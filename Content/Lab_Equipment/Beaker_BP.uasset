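; Beaker lab-equipment Blueprint containing a battery-limited light, built from a Cylinder and a PointLight.
; The Light input flips LightStatus through a FlipFlop and shows both components if the charge flag NewVar0 is set.
; Tick restarts a 0.2-second retriggerable delay, then, while lit, decrements the charge and updates NewVar0.
; Both visibility calls, including the empty-battery one, set visible to true, so nothing here hides the light.
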(event `InputAction|Light`
  (params (Key :type "Key Structure"))
  (:`Pressed`
    (bind _isa (`/Engine/EditorBlueprintResources/StandardMacros.FlipFlop`)
      (:`A`
        _)
      (:`B`
        _))
    (set `self.LightStatus` _isa)
    (if (`self.NewVar_0`)
      (`SceneComponent.SetVisibility` (`self.Cylinder`) true false)
      (`SceneComponent.SetVisibility` (`self.PointLight`) true false))))

(event `self.ReceiveTick`
  (params (DeltaSeconds :type "Float (single-precision)"))
  (`KismetSystemLibrary.RetriggerableDelay` 0.2)
  (if (`self.LightStatus`)
    (bind _result (`/Engine/EditorBlueprintResources/StandardMacros.DecrementFloat` (`self.Value 1`))
      (:`  `
        (bind _output_get (set `self.Amount of Battery` _result))
        (bind _output_get_2 (set `self.NewVar_0` (>= _output_get 0.01)))
        (if (not _output_get_2)
          (`SceneComponent.SetVisibility` (`self.Cylinder`) true false)
          (`SceneComponent.SetVisibility` (`self.PointLight`) true false))))))

(fn `UserConstructionScript`)